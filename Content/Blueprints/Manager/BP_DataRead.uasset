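; BP_DataRead records TCP scenario messages and plays them back onto BP_Node actors, live or as a replay.
; The first JSON message sets up BP_Manager's existing nodes by PlatformID and fills the PIP camera selectors.
; Tick then applies the latest, next or slider-chosen frame's position and attitude, enabling the slider at ScenarioEnd.
; Trail colors follow UI tints by object type; the older node-spawning path is unused.
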(event `TrailColor`
  ;[1 1 1] Tail Color
  (bind _asbp_game_mode_gps (cast `/Game/Blueprints/Framework/BP_GameMode_GPS` (`GameplayStatics.GetGameMode`)))
  (for _array_element (`self.Out Actors`)
    (bind _asbp_node (cast `/Game/Blueprints/Manager/BP_Node` _array_element))
    (bind _objecttype (`/Game/Blueprints/Manager/BP_Node.ObjectType` _asbp_node))
    (if (`|EnumEquality` _objecttype "NewEnumerator0")
      (bind _dyamat_trail (`/Game/Blueprints/Manager/BP_Node.DyaMat_Trail` _asbp_node))
      (bind _gameui (`/Game/Blueprints/Framework/BP_GameMode_GPS.GameUI` _asbp_game_mode_gps))
      (bind (_brush_imagesize _brush_margin _brush_tintcolor) (break `SlateBrush` (`Image.Brush` (`/Game/Blueprints/Widget/GameMenu.Image_Friend` _gameui))))
      (`MaterialInstanceDynamic.SetVectorParameterValue` _dyamat_trail "Color" (`.SpecifiedColor` (break `SlateColor` _brush_tintcolor)))
      (elif (`|EnumEquality` _objecttype "NewEnumerator1")
        (bind (_brush_imagesize_2 _brush_margin_2 _brush_tintcolor_2) (break `SlateBrush` (`Image.Brush` (`/Game/Blueprints/Widget/GameMenu.Image_FriendMissile` _gameui))))
        (bind _specifiedcolor (break `SlateColor` _brush_tintcolor_2))
        (`MaterialInstanceDynamic.SetVectorParameterValue` _dyamat_trail "Color" _specifiedcolor)
        (elif (`|EnumEquality` _objecttype "NewEnumerator2")
          (`MaterialInstanceDynamic.SetVectorParameterValue` _dyamat_trail "Color" _specifiedcolor)
          (elif (`|EnumEquality` _objecttype "NewEnumerator3")
            (bind (_brush_imagesize_3 _brush_margin_3 _brush_tintcolor_3) (break `SlateBrush` (`Image.Brush` (`/Game/Blueprints/Widget/GameMenu.Image_Enemy` _gameui))))
            (`MaterialInstanceDynamic.SetVectorParameterValue` _dyamat_trail "Color" (`.SpecifiedColor` (break `SlateColor` _brush_tintcolor_3)))
            (elif true
              (bind (_brush_imagesize_4 _brush_margin_4 _brush_tintcolor_4) (break `SlateBrush` (`Image.Brush` (`/Game/Blueprints/Widget/GameMenu.Image_EnemyMissile` _gameui))))
              (`MaterialInstanceDynamic.SetVectorParameterValue` _dyamat_trail "Color" (`.SpecifiedColor` (break `SlateColor` _brush_tintcolor_4))))))))))

(event `self.ReceiveBeginPlay`
  ;[1 1 1] Read Data From TCP
  (bind _returnvalue (`GameplayStatics.GetActorOfClass` "/Game/Blueprints/Manager/BP_Manager.BP_Manager_C"))
  (set `self.Out Actors` (`/Game/Blueprints/Manager/BP_Manager.Out Actors` _returnvalue))
  (`KismetArrayLibrary.Array_Clear` (`self.DataArray`))
  (bind _asbp_game_instance (cast `/Game/Blueprints/Framework/BP_GameInstance` (`GameplayStatics.GetGameInstance`)))
  (if (`KismetStringLibrary.NotEqual_StrStr` (`/Game/Blueprints/Framework/BP_GameInstance.TCPConnection` _asbp_game_instance))
    (add `SocketClientBPLibrary.onreceiveTCPMessageEventDelegate` (`SocketClientBPLibrary.getSocketClientTarget`) (delegate `CustomEvent_1`))))

(event `CustomEvent_1`
  (params (message :type String) (byteArray :type "Array of Byte (by ref)") (clientConnectionID :type String))
  ;[1 1 1] Read Data From TCP
  (`KismetArrayLibrary.Array_Add` (`self.DataArray`) message))

(event `self.ReceiveTick`
  (params (DeltaSeconds :type "Float (single-precision)"))
  (bind _dataarray (`self.DataArray`))
  (bind _gameui (`self.GameUI`))
  (bind _returnvalue (`KismetArrayLibrary.Array_LastIndex` (`self.DataArray`)))
  (`|ExecutionSequence`
    (:`then_0`
      (`self.GameUI`
        (:`then`)
        (:`else`
          (bind _asbp_game_mode_gps (cast `/Game/Blueprints/Framework/BP_GameMode_GPS` (`GameplayStatics.GetGameMode`)))
          (set `self.GameUI` (`/Game/Blueprints/Framework/BP_GameMode_GPS.GameUI` _asbp_game_mode_gps)))))
    (:`then_1`
      (if (`self.IsLoaded`)
        (`self.GameUI`
          (:`then`
            (if (`/Game/Blueprints/Widget/GameMenu.IsReplaySliderChange` (`self.GameUI`))
              (set `/Game/Blueprints/Widget/GameMenu.PlayState` "NewEnumerator0" _gameui)
              (set `self.Index` (`KismetMathLibrary.FTrunc` (* (- (`KismetArrayLibrary.Array_Length` (`self.DataArray`)) 1) (`Slider.GetNormalizedValue` (`/Game/Blueprints/Widget/GameMenu.Slider_Replay` _gameui)))))
              (else
                (switch `/Game/Blueprints/State/E_PlayState` (`/Game/Blueprints/Widget/GameMenu.PlayState` _gameui)
                  (:`NewEnumerator0`
                    _)
                  (:`NewEnumerator2`
                    (set `self.Index` 0)))
                (if (`CheckBox.IsChecked` (`/Game/Blueprints/Widget/GameMenu.CheckBox_Realtime` _gameui))
                  (set `self.Index` _returnvalue)
                  (else
                    (bind _result (`/Engine/EditorBlueprintResources/StandardMacros.IncrementInt` (`self.Index`))
                      (:`  `
                        (if (> _result _returnvalue)
                          (set `self.Index` _returnvalue))))))))
            (bind _returnvalue_2 (`JSONParserBPLibrary.JsonStringToObject` (`|GetArrayItem` (`self.DataArray`) (`self.Index`))))
            (bind (_objectmap _boolmap) (`JSONParserBPLibrary.BreakJson_Object` _returnvalue_2))
            (bind (_value _returnvalue_3) (`BlueprintMapLibrary.Map_Find` _objectmap "PlatformDatas"))
            (if _returnvalue_3
              (bind (_objectmap_2 _boolmap_2 _numbermap _stringmap _objectarray) (`JSONParserBPLibrary.BreakJson_Object` _value))
              (for _array_element _objectarray
                (bind (_objectmap_3 _boolmap_3 _numbermap_2) (`JSONParserBPLibrary.BreakJson_Object` _array_element))
                (bind _asbp_node (cast `/Game/Blueprints/Manager/BP_Node` (`BlueprintMapLibrary.Map_Find` (`self.ActorMap`) (`KismetMathLibrary.FTrunc` (`BlueprintMapLibrary.Map_Find` _numbermap_2 "PlatformID")))))
                (set `/Game/Blueprints/Manager/BP_Node.Lat` (`BlueprintMapLibrary.Map_Find` _numbermap_2 "Lat") _asbp_node)
                (set `/Game/Blueprints/Manager/BP_Node.Lon` (`BlueprintMapLibrary.Map_Find` _numbermap_2 "Lon") _asbp_node)
                (set `/Game/Blueprints/Manager/BP_Node.Pitch` (`BlueprintMapLibrary.Map_Find` _numbermap_2 "Pitch") _asbp_node)
                (set `/Game/Blueprints/Manager/BP_Node.Roll` (`BlueprintMapLibrary.Map_Find` _numbermap_2 "Roll") _asbp_node)
                (set `/Game/Blueprints/Manager/BP_Node.Yaw` (`BlueprintMapLibrary.Map_Find` _numbermap_2 "Yaw") _asbp_node)
                (set `/Game/Blueprints/Manager/BP_Node.Alt` (`BlueprintMapLibrary.Map_Find` _numbermap_2 "Alt") _asbp_node)
                (set `/Game/Blueprints/Manager/BP_Node.Time` (`BlueprintMapLibrary.Map_Find` _numbermap_2 "Time") _asbp_node)
                (`/Game/Blueprints/Manager/BP_Node.SetFirstPos` _asbp_node))
              (elif (`BlueprintMapLibrary.Map_Find` _boolmap "ScenarioEnd")
                (`Widget.SetIsEnabled` (`/Game/Blueprints/Widget/GameMenu.Slider_Replay` (`self.GameUI`)) true))))
          (:`else`))
        (else
          ;[1 1 1] Create Objects
          (if (> (`KismetArrayLibrary.Array_Length` _dataarray) 0)
            (`/Engine/EditorBlueprintResources/StandardMacros.DoOnce` false
              (:`Completed`
                (bind _returnvalue_4 (`JSONParserBPLibrary.JsonStringToObject` (`|GetArrayItem` _dataarray)))
                (bind _objectmap_4 (`JSONParserBPLibrary.BreakJson_Object` _returnvalue_4))
                (bind (_objectmap_5 _boolmap_4 _numbermap_3) (`JSONParserBPLibrary.BreakJson_Object` (`BlueprintMapLibrary.Map_Find` _objectmap_4 "ScenarioInitialization")))
                (set `self.Ref_Lat` (`BlueprintMapLibrary.Map_Find` _numbermap_3 "RefLat"))
                (set `self.Ref_Lon` (`BlueprintMapLibrary.Map_Find` _numbermap_3 "RefLon"))
                (bind (_objectmap_6 _boolmap_5 _numbermap_4 _stringmap_2 _objectarray_2) (`JSONParserBPLibrary.BreakJson_Object` (`BlueprintMapLibrary.Map_Find` _objectmap_4 "Platforms")))
                (for _array_element_2 _objectarray_2
                  (bind (_objectmap_7 _boolmap_6 _numbermap_5 _stringmap_3) (`JSONParserBPLibrary.BreakJson_Object` _array_element_2))
                  (bind _returnvalue_5 (`KismetMathLibrary.FTrunc` (`BlueprintMapLibrary.Map_Find` _numbermap_5 "PlatformID")))
                  (bind _output (`|GetArrayItem` (`self.Out Actors`) (- _returnvalue_5 1)))
                  (bind _asbp_node_2 (cast `/Game/Blueprints/Manager/BP_Node` _output))
                  (set `/Game/Blueprints/Manager/BP_Node.RefLat` (`self.Ref_Lat`) _asbp_node_2)
                  (set `/Game/Blueprints/Manager/BP_Node.RefLon` (`self.Ref_Lon`) _asbp_node_2)
                  (bind _value_2 (`BlueprintMapLibrary.Map_Find` _stringmap_3 "PlatformName"))
                  (set `/Game/Blueprints/Manager/BP_Node.PlatformName` _value_2 _asbp_node_2)
                  (`BlueprintMapLibrary.Map_Add` (`self.ActorMap`) _returnvalue_5 _asbp_node_2)
                  (bind _asobject_info (cast `/Game/Blueprints/Widget/Util/ObjectInfo` (`WidgetComponent.GetUserWidgetObject` (`self.GetComponentByClass` _output "/Script/UMG.WidgetComponent"))))
                  (`TextBlock.SetText` (`/Game/Blueprints/Widget/Util/ObjectInfo.Text_Name` _asobject_info) (`KismetTextLibrary.Conv_StringToText` _value_2))
                  (`/Game/Blueprints/Manager/BP_Node.SetViz` _asbp_node_2 true)
                  (`/Game/Blueprints/Manager/BP_Node.SetCollision` _asbp_node_2))
                (`self.DataReadEnd`)
                (set `self.IsLoaded` true)
                (bind _asbp_game_mode_gps_2 (cast `/Game/Blueprints/Framework/BP_GameMode_GPS` (`GameplayStatics.GetGameMode`)))
                (bind _verticalbox_pip (`/Game/Blueprints/Widget/GameMenu.VerticalBox_PIP` (`/Game/Blueprints/Framework/BP_GameMode_GPS.GameUI` _asbp_game_mode_gps_2)))
                (for (_array_element_3 _array_index) (`PanelWidget.GetAllChildren` _verticalbox_pip)
                  (bind _aspip_widget (cast `/Game/Blueprints/Widget/Util/PIP/PIP_Widget` _array_element_3))
                  (bind _values (`BlueprintMapLibrary.Map_Values` (`self.ActorMap`)))
                  (for _array_element_4 _values
                    (bind _asbp_node_3 (cast `/Game/Blueprints/Manager/BP_Node` _array_element_4))
                    (bind _objecttype (`/Game/Blueprints/Manager/BP_Node.ObjectType` _asbp_node_3))
                    (if (or (or (`|EnumEquality` _objecttype "NewEnumerator0") (`|EnumEquality` _objecttype "NewEnumerator1")) (or (`|EnumEquality` _objecttype "NewEnumerator2") (`|EnumEquality` _objecttype "NewEnumerator3")))
                      (bind _combobox_pip (`/Game/Blueprints/Widget/Util/PIP/PIP_Widget.ComboBox_PIP` _aspip_widget))
                      (`ComboBoxString.AddOption` _combobox_pip (`/Game/Blueprints/Manager/BP_Node.PlatformName` _asbp_node_3))))
                  (`ComboBoxString.SetSelectedIndex` _combobox_pip _array_index))
                (`Widget.SetVisibility` _verticalbox_pip "SelfHitTestInvisible")))))))
    (:`then_2`
      (`KismetSystemLibrary.Delay` 0.5)
      (`self.TrailColor`))))

(fn `UserConstructionScript`)