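; Manager Blueprint that optionally starts a demo sequence and exports node logs as a SIMDIS ASI scenario file.
; On BeginPlay it plays a level sequence if the game instance's IsDemo flag is set.
; SaveLog builds platform headers and concatenates recorded data from BP_Node actors, adds version and reference-coordinate initialization, then saves the text under the current level's name.
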(event `self.ReceiveBeginPlay`
  (bind _asbp_game_instance (cast `/Game/Blueprints/Framework/BP_GameInstance` (`GameplayStatics.GetGameInstance`)))
  (bind _output_get (set `self.IsDemo` (`/Game/Blueprints/Framework/BP_GameInstance.IsDemo` _asbp_game_instance)))
  (if _output_get
    (`MovieSceneSequencePlayer.Play` (`LevelSequenceActor.SequencePlayer` (`self.LevelSequnce`)))))

(event `SaveLog`
  (bind (_arrayindex _arrayelement) (`/Engine/EditorBlueprintResources/StandardMacros.ReverseForEachLoop` (`self.Out Actors`))
    (:`LoopBody`
      (bind _asbp_node (cast `/Game/Blueprints/Manager/BP_Node` _arrayelement))
      (bind _returnvalue (`KismetStringLibrary.Conv_IntToString` (`/Game/Blueprints/Manager/BP_Node.PlatformID` _asbp_node)))
      (set `self.PlatformHeaderString` (`KismetStringLibrary.Concat_StrStr` (`KismetStringLibrary.Concat_StrStr` "PlatformID " _returnvalue " \n" "PlatformName " _returnvalue " \"" (`/Game/Blueprints/Manager/BP_Node.PlatformName` _asbp_node) "\" \n" "PlatformIcon " _returnvalue " \"" (`/Game/Blueprints/Manager/BP_Node.PlatformIcon` _asbp_node) "\" \n") (`self.PlatformHeaderString`))))
    (:`Completed`
      (for _array_element (`self.Out Actors`)
        (bind _asbp_node_2 (cast `/Game/Blueprints/Manager/BP_Node` _array_element))
        (set `self.NodeData` (`KismetStringLibrary.Concat_StrStr` (`self.NodeData`) (`/Game/Blueprints/Manager/BP_Node.OutData` _asbp_node_2))))
      (bind _returnvalue_2 (`GameplayStatics.GetCurrentLevelName` true))
      (`FileManagerBFL.SaveTxt` (`KismetStringLibrary.Concat_StrStr` (`KismetStringLibrary.Concat_StrStr` "# SIMDIS Ascii Scenario Input (ASI) File Format \n \n# Scenario Initialization \n \n" "Version " (`self.Version`) " \n" "RefLat " (`self.RefLat`) " \n" "RefLon " (`self.RefLon`) " \n" "CoordSystem \"LLA\" \nDegreeAngles 1 \n \n" "# Platform Header  \n \n" (`self.PlatformHeaderString`)) " \n# Platform Data \n \n \n# PlatformData PlatformID Time Lat Lon Alt Yow Pitch Roll  \n \n" (`self.NodeData`)) (`KismetStringLibrary.Concat_StrStr` _returnvalue_2 ".asi"))
      (`KismetSystemLibrary.PrintString` "Save Log" true true (struct :`R` 0.994846 :`G` 1.0 :`A` 1.0) 5.0))))

(fn `UserConstructionScript`)