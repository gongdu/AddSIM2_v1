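; BP_Node is a military simulation platform actor driven by BP_Manager's demo flag.
; In demo mode, one node type follows a spline or target, and nodes append geographic pose logs; otherwise they replay lat/lon/alt and attitude through UTM conversion.
; That type's collisions trigger explosions and send hit JSON over TCP.
; Events provide chaff, radar scaling, CIWS bursts and render-target picture-in-picture views.
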(event `self.ReceiveBeginPlay`
  (bind _returnvalue (`KismetMathLibrary.RandomFloatInRange` 0.0 0.5))
  (bind _traileffect (`self.TrailEffect`))
  ;[1 1 1] 초기화
  (bind _returnvalue_2 (`GameplayStatics.GetActorOfClass` "/Game/Blueprints/Manager/BP_Manager.BP_Manager_C"))
  (set `self.DataManager` _returnvalue_2)
  (bind _returnvalue_3 (`PrimitiveComponent.CreateDynamicMaterialInstance` _traileffect 0 (`PrimitiveComponent.GetMaterial` _traileffect 0) "None"))
  (set `self.DyaMat_Trail` _returnvalue_3)
  (if (`/Game/Blueprints/Manager/BP_Manager.IsDemo` (`self.DataManager`))
    (set `self.DeltaPos` (`KismetMathLibrary.MakeVector` (`KismetMathLibrary.RandomFloatInRange` 30.0 50.0) _returnvalue _returnvalue))
    (`ActorComponent.SetActive` (`self.TrailEffect`) true false)
    (`self.SetCollision`)
    (if (`self.isSplineMove`)
      (set `self.Spline` (`self.GetComponentByClass` (`self.Guide`) "/Script/Engine.SplineComponent")))))

(event `self.SphereCollision.OnComponentHit`
  (params (HitComponent :type "PrimitiveComponent Object Reference") (OtherActor :type "Actor Object Reference") (OtherComp :type "PrimitiveComponent Object Reference") (NormalImpulse :type "Vector Structure") (Hit :type "HitResult Structure (by ref)"))
  (bind (_bblockinghit _binitialoverlap _time _distance _location _impactpoint) (`GameplayStatics.BreakHitResult` Hit))
  (bind _returnvalue (`self.GetParentActor` OtherActor))
  (bind (_bblockinghit_2 _binitialoverlap_2 _time_2 _distance_2 _location_2 _impactpoint_2 _normal _impactnormal _physmat _hitactor) (`GameplayStatics.BreakHitResult` Hit))
  ;[1 1 1] Collision Check
  (`KismetSystemLibrary.PrintString` (`KismetSystemLibrary.GetDisplayName` OtherActor))
  (if (`|EnumEquality` (`self.NodeType`) "NewEnumerator2")
    (`/Engine/EditorBlueprintResources/StandardMacros.IsValid` _returnvalue
      (:`Is Valid`
        (bind _asbp_node (cast `/Game/Blueprints/Manager/BP_Node` _returnvalue)
          (:`then`
            (`self.Explosion` _asbp_node)
            (`GameplayStatics.SpawnEmitterAtLocation` "/Game/Effects/M5VFXVOL2/Particles/Explosion/Fire_Exp_Big_00.Fire_Exp_Big_00" _impactpoint (struct) (3.0 3.0 3.0) :!label _label)
            (`self.SetActorEnableCollision` false)
            (`SceneComponent.SetVisibility` (`self.ChildActor1`) false false)
            (set `self.IsHit` true)
            (`KismetSystemLibrary.DrawDebugSphere` _impactpoint 50.0 12 (struct :`R` 1.0 :`B` 0.175133 :`A` 1.0) 60.0)
            (bind _returnvalue_2 (`JSONParserBPLibrary.MakeJson_Object` :`StringMap` (`JSONParserBPLibrary.MakeMapString` "Name" (`KismetSystemLibrary.GetDisplayName` _hitactor))))
            (bind _returnvalue_3 (`JSONParserBPLibrary.MakeJson_Object` :`NumberMap` (`JSONParserBPLibrary.AddMapNumber` (`JSONParserBPLibrary.AddMapNumber` (`JSONParserBPLibrary.MakeMapNumber` "X " (.x _impactpoint_2)) "Y" (.y _impactpoint_2)) "Z" (.z _impactpoint_2))))
            (bind _returnvalue_4 (`JSONParserBPLibrary.MakeJson_Object` :`NumberMap` (`JSONParserBPLibrary.AddMapNumber` (`JSONParserBPLibrary.AddMapNumber` (`JSONParserBPLibrary.MakeMapNumber` "X " (.x _impactnormal)) "Y" (.y _impactnormal)) "Z" (.z _impactnormal))))
            (bind _returnvalue_5 (`JSONParserBPLibrary.MakeJson_Object` (`JSONParserBPLibrary.AddMapObject` (`JSONParserBPLibrary.AddMapObject` (`JSONParserBPLibrary.MakeMapObject` "HIt Object" _returnvalue_2) "Hit Position" _returnvalue_3) "Hit Direction" _returnvalue_4)))
            (bind _returnvalue_6 (`JSONParserBPLibrary.JsonObjectToString` _returnvalue_5))
            (bind _asbp_game_instance (cast `/Game/Blueprints/Framework/BP_GameInstance` (`GameplayStatics.GetGameInstance`)))
            (bind _tcpconnection (`/Game/Blueprints/Framework/BP_GameInstance.TCPConnection` _asbp_game_instance))
            (bind _returnvalue_7 (`SocketClientBPLibrary.isTCPConnected` (`SocketClientBPLibrary.getSocketClientTarget`) _tcpconnection))
            (if _returnvalue_7
              (`SocketClientBPLibrary.socketClientSendTCP` :`self` (`SocketClientBPLibrary.getSocketClientTarget`) :`connectionID` _tcpconnection :`message` _returnvalue_6 :`addLineBreak` false)
              (`KismetSystemLibrary.PrintString` "Collision Send!!" true true (struct :`R` 0.279998 :`G` 1.0 :`B` 0.022275 :`A` 1.0) 10.0)
              (else
                (`KismetSystemLibrary.PrintString` "Not connected." true true (struct :`R` 1.0 :`G` 0.120146 :`B` 0.060419 :`A` 1.0)))))
          (:`CastFailed`
            (`KismetSystemLibrary.PrintString` "Hello"))))
      (:`Is Not Valid`
        (goto _label)))))

(event `SetFirstPos`
  ;[1 1 1] 처음 위치 이동
  (`/Engine/EditorBlueprintResources/StandardMacros.DoOnce` false
    (:`Completed`
      (`KismetSystemLibrary.Delay` 1.0)
      (set `self.IsFirstMove` false)
      (`KismetSystemLibrary.Delay` 5.0)
      (`ActorComponent.SetActive` (`self.TrailEffect`) true false))))

(event `self.ReceiveTick`
  (params (DeltaSeconds :type "Float (single-precision)"))
  (bind (_returnvalue_roll _returnvalue_pitch _returnvalue_yaw) (`KismetMathLibrary.BreakRotator` (`self.K2_GetActorRotation`)))
  (bind _returnvalue (`GameplayStatics.GetWorldDeltaSeconds`))
  (bind _spline (`self.Spline`))
  (bind _springarm (`self.SpringArm`))
  (bind (_returnvalue_x _returnvalue_y _returnvalue_z) (`KismetMathLibrary.BreakVector` (/ (`self.K2_GetActorLocation`) 100.0)))
  (bind (_utmnorthing _utmeasting) (`UTMConverter.LLtoUTM` (`self.Lat`) (`self.Lon`)))
  (bind (_utmnorthing_2 _utmeasting_2 _utmzone) (`UTMConverter.LLtoUTM` (`self.RefLat`) (`self.RefLon`)))
  (bind (_utmnorthing_3 _utmeasting_3) (`UTMConverter.LLtoUTM` (`self.RefLat`) (`self.RefLon`)))
  (bind _returnvalue_2 (`KismetStringLibrary.ParseIntoArray` (`KismetStringLibrary.Conv_DoubleToString` (`self.DataTime`)) "."))
  (bind _returnvalue_3 (* (`self.SplineDistance`) (`SplineComponent.GetSplineLength` (`self.Spline`))))
  (bind (_lat _long) (`UTMConverter.UTMtoLL` (+ _utmnorthing_2 _returnvalue_y) (+ _utmeasting_2 _returnvalue_x) _utmzone))
  (bind (_returnvalue_x_2 _returnvalue_y_2 _returnvalue_z_2) (`KismetMathLibrary.BreakVector` (* (`KismetMathLibrary.MakeVector` (* -1 (- _utmeasting_3 _utmeasting)) (- _utmnorthing _utmnorthing_3) (`self.Alt`)) 100.0)))
  (bind _returnvalue_4 (`KismetMathLibrary.MakeVector` _returnvalue_x_2 _returnvalue_y_2 _returnvalue_z_2))
  (if (`/Game/Blueprints/Manager/BP_Manager.IsDemo` (`self.DataManager`))
    (`|ExecutionSequence`
      (:`then_0`
        (if (`|EnumEquality` (`self.NodeType`) "NewEnumerator2")
          (if (`self.IsHit`)
            _
            (elif (`self.isSplineMove`)
              ;[1 1 1] Spline Move
              (`self.K2_SetActorLocation` (`SplineComponent.GetLocationAtDistanceAlongSpline` _spline _returnvalue_3 "World"))
              (`self.K2_SetActorRotation` (`SplineComponent.GetRotationAtDistanceAlongSpline` _spline _returnvalue_3 "Local"))
              (else
                ;[1 1 1] Target Move
                (`self.K2_SetActorRotation` (`KismetMathLibrary.Conv_VectorToRotator` (`KismetMathLibrary.Normal` (- (`self.K2_GetActorLocation` (`self.TargetActor`)) (`self.K2_GetActorLocation`)))))
                (`self.K2_SetActorLocation` (`KismetMathLibrary.VLerp` (`self.K2_GetActorLocation`) (`self.K2_GetActorLocation` (`self.TargetActor`)) (`self.TargetLerp`))))))))
      (:`then_1`
        ;[1 1 1] Write Log
        (`KismetSystemLibrary.Delay` (`self.DelayTime`))
        (set `self.OutData` (`KismetStringLibrary.Concat_StrStr` (`self.OutData`) (`KismetStringLibrary.Concat_StrStr` "PlatformData " "" (`KismetStringLibrary.Conv_IntToString` (`self.PlatformID`)) " " (`KismetStringLibrary.Concat_StrStr` (`KismetStringLibrary.Concat_StrStr` (`|GetArrayItem` _returnvalue_2) "." (`KismetStringLibrary.GetSubstring` (`|GetArrayItem` _returnvalue_2 1) 0 2)) " " (`KismetStringLibrary.Conv_DoubleToString` _lat) " " (`KismetStringLibrary.Conv_DoubleToString` _long) " " (`KismetStringLibrary.Conv_DoubleToString` _returnvalue_z) " " (`KismetStringLibrary.Conv_DoubleToString` (+ _returnvalue_yaw 90.0)) " " (`KismetStringLibrary.Conv_DoubleToString` _returnvalue_pitch) " " (`KismetStringLibrary.Conv_DoubleToString` _returnvalue_roll) " \n"))))
        (set `self.DataTime` (+ (`self.DataTime`) (`self.DelayTime`)))))
    (else
      (`|ExecutionSequence`
        (:`then_0`
          ;[1 1 1] 카메라 조정
          (if (`self.CanCameraMove`)
            (bind _asbp_default_pawn_gps_a2s (cast `/Game/Blueprints/Framework/BP_DefaultPawn_GPS_A2S` (`GameplayStatics.GetPlayerPawn` 0)))
            (set `SpringArmComponent.TargetArmLength` (`KismetMathLibrary.FClamp` (+ (`SpringArmComponent.TargetArmLength` _springarm) (`/Game/Blueprints/Framework/BP_DefaultPawn_GPS_A2S.ZoomValue` _asbp_default_pawn_gps_a2s)) 100.0 20000.0) _springarm)
            (`SceneComponent.K2_SetRelativeRotation` (`self.SpringArm`) (`Controller.GetControlRotation` (`GameplayStatics.GetPlayerController` 0)) false false)))
        (:`then_1`
          ;[1 1 1] Read Log
          (if (not (`self.IsHit`))
            (`|ExecutionSequence`
              (:`then_0`
                (`self.K2_SetActorRotation` (`KismetMathLibrary.RLerp` (`self.K2_GetActorRotation`) (`KismetMathLibrary.MakeRotator` (+ (`self.Roll`) 0.0) (+ (`self.Pitch`) 0.0) (+ (`self.Yaw`) -90.0)) (`KismetMathLibrary.FClamp` (* _returnvalue 2.0)) true)))
              (:`then_1`
                (if (`|EnumInequality` (`self.NodeType`) "NewEnumerator1")
                  (`self.K2_SetActorLocation` (`KismetMathLibrary.MakeVector` (.x (select `bool` (`self.IsFirstMove`) :`false` _returnvalue_4 :`true` (`KismetMathLibrary.VLerp` (`self.K2_GetActorLocation`) _returnvalue_4 _returnvalue))) (.y (select `bool` (`self.IsFirstMove`) :`false` _returnvalue_4 :`true` (`KismetMathLibrary.VLerp` (`self.K2_GetActorLocation`) _returnvalue_4 _returnvalue))) (.z (select `bool` (`self.IsFirstMove`) :`false` _returnvalue_4 :`true` (`KismetMathLibrary.VLerp` (`self.K2_GetActorLocation`) _returnvalue_4 _returnvalue))))))))))))))

(event `SetChaff`
  ;[1 1 1] Chaff
  (`SceneComponent.SetVisibility` (`self.ChildActor1`) false false)
  (`GameplayStatics.SpawnEmitterAtLocation` (`self.FireEmitter`) (`self.K2_GetActorLocation`)))

(event `SetRadar`
  ;[1 1 1] Radar
  (`iTween.ActorScaleFromToSimple` "RadarTween" (`ChildActorComponent.ChildActor` (`self.ChildActor1`)) (0.0 0.0 0.0) (3000.0 3000.0 3000.0) false 5.0 "linear" "" null null null self))

(event `iTInterface.OnTweenComplete`
  (params (eventOperator :type "iTweenEvent Object Reference") (actorTweening :type "Actor Object Reference") (componentTweening :type "SceneComponent Object Reference") (widgetTweening :type "Widget Object Reference") (tweenName :type Name) (sweepHitResultForMoveEvents :type "HitResult Structure") (successfulTransform :type Boolean))
  ;[1 1 1] Radar
  (switch `name` tweenName
    (:`RadarTween`
      (`SceneComponent.SetVisibility` (`self.ChildActor1`) false false))))

(event `Explosion`
  ;[1 1 1] Explosion
  (for _array_element (`self.ExpEmitterArray`)
    (`ActorComponent.SetActive` (`Emitter.ParticleSystemComponent` _array_element) true false)))

(event `SetCollision`
  (bind _objecttype (`self.ObjectType`))
  (bind _spherecollision (`self.SphereCollision`))
  ;[1 1 1] Collision
  (`KismetSystemLibrary.Delay` 3.0)
  (`|ExecutionSequence`
    (:`then_0`
      (if (`|EnumEquality` _objecttype "NewEnumerator0")
        (`PrimitiveComponent.SetCollisionProfileName` _spherecollision "Blue" false)
        (elif (`|EnumEquality` _objecttype "NewEnumerator1")
          (`PrimitiveComponent.SetCollisionProfileName` _spherecollision "BlueGun" false)
          (elif (`|EnumEquality` _objecttype "NewEnumerator2")
            (`PrimitiveComponent.SetCollisionProfileName` _spherecollision "Red" false)
            (elif (`|EnumEquality` _objecttype "NewEnumerator3")
              (`PrimitiveComponent.SetCollisionProfileName` _spherecollision "RedGun" false))))))
    (:`then_1`
      (if (`|EnumEquality` (`self.NodeType`) "NewEnumerator2")
        (`PrimitiveComponent.SetSimulatePhysics` _spherecollision true)))))

(event `Fire`
  ;[1 1 1] Fire
  (set `self.MaxMultiFire` (`KismetMathLibrary.RandomIntegerInRange` 10 15))
  (bind _returnvalue (`KismetSystemLibrary.K2_SetTimerDelegate` (delegate `MultiFire`) 0.2 true)))

(event `MultiFire`
  (bind _ciws_ref (`self.ciws_ref`))
  ;[1 1 1] Fire
  (`GameplayStatics.SpawnEmitterAtLocation` (`self.FireEmitter`) (`SceneComponent.K2_GetComponentLocation` _ciws_ref) (`SceneComponent.K2_GetComponentRotation` _ciws_ref))
  (bind _result (`/Engine/EditorBlueprintResources/StandardMacros.DecrementInt` (`self.MaxMultiFire`))
    (:`  `
      (if (<= _result 0)
        (`KismetSystemLibrary.K2_ClearAndInvalidateTimerHandle` (stale `Fire` _returnvalue))))))

(event `SetViz`
  (params (IsShow :type Boolean))
  (bind _scenecapturecomponent2d (`self.SceneCaptureComponent2D`))
  ;[1 1 1] PIP
  (`SceneComponent.SetVisibility` (`self.W_info`) IsShow false)
  (if IsShow
    (bind _returnvalue (`KismetRenderingLibrary.CreateRenderTarget2D` 256))
    (bind _output_get (set `self.RenderTexture` _returnvalue))
    (set `SceneCaptureComponent2D.TextureTarget` _output_get _scenecapturecomponent2d)
    (`SceneComponent.SetVisibility` _scenecapturecomponent2d true false)
    (`ActorComponent.SetActive` _scenecapturecomponent2d true false)
    (bind _returnvalue_2 (`|CreateWidget` "/Game/Blueprints/Widget/Util/PIP/PIP_Widget.PIP_Widget_C"))
    (bind _returnvalue_3 (`KismetMaterialLibrary.CreateDynamicMaterialInstance` "/Game/Blueprints/Widget/Util/PIP/M_PIP.M_PIP"))
    (`MaterialInstanceDynamic.SetTextureParameterValue` _returnvalue_3 "Texture" (`self.RenderTexture`))
    (`Image.SetBrushFromMaterial` (`/Game/Blueprints/Widget/Util/PIP/PIP_Widget.Image_Render` _returnvalue_2) _returnvalue_3)
    (set `/Game/Blueprints/Widget/Util/PIP/PIP_Widget.ViewTarget` self _returnvalue_2)))

(fn `UserConstructionScript`
  (bind _returnvalue (`GameplayStatics.GetActorOfClass` "/Game/Blueprints/Manager/BP_Manager.BP_Manager_C"))
  (set `self.DataManager` _returnvalue))