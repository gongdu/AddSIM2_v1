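; BP_Node is an actor representing a geo-referenced platform, placed by latitude, longitude and altitude.
; Outside demo mode, Tick converts coordinates to UTM offsets from a reference point, smooths rotation, and drives spring-arm zoom and rotation from the player.
; In demo mode, it instead appends delayed, timestamped pose records in lat/long to OutData.
; A hit freezes movement, draws a debug sphere and sends JSON impact details over the GameInstance's TCP connection.
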(event `self.ReceiveBeginPlay`
  (bind _traileffect (`self.TrailEffect`))
  (bind _returnvalue (`PrimitiveComponent.CreateDynamicMaterialInstance` _traileffect 0 (`PrimitiveComponent.GetMaterial` _traileffect 0) "None"))
  (set `self.DyaMat_Trail` _returnvalue))

(event `self.ReceiveHit`
  (params (MyComp :type "PrimitiveComponent Object Reference") (Other :type "Actor Object Reference") (OtherComp :type "PrimitiveComponent Object Reference") (bSelfMoved :type Boolean) (HitLocation :type "Vector Structure") (HitNormal :type "Vector Structure") (NormalImpulse :type "Vector Structure") (Hit :type "HitResult Structure (by ref)"))
  (bind (_bblockinghit _binitialoverlap _time _distance _location _impactpoint _normal _impactnormal _physmat _hitactor) (`GameplayStatics.BreakHitResult` Hit))
  (set `self.IsHit` true)
  (`KismetSystemLibrary.DrawDebugSphere` HitLocation 50.0 12 (struct :`R` 1.0 :`B` 0.175133 :`A` 1.0) 60.0)
  (bind _returnvalue (`JSONParserBPLibrary.MakeJson_Object` :`StringMap` (`JSONParserBPLibrary.MakeMapString` "Name" (`KismetSystemLibrary.GetDisplayName` _hitactor))))
  (bind _returnvalue_2 (`JSONParserBPLibrary.MakeJson_Object` :`NumberMap` (`JSONParserBPLibrary.AddMapNumber` (`JSONParserBPLibrary.AddMapNumber` (`JSONParserBPLibrary.MakeMapNumber` "X " (.x _impactpoint)) "Y" (.y _impactpoint)) "Z" (.z _impactpoint))))
  (bind _returnvalue_3 (`JSONParserBPLibrary.MakeJson_Object` :`NumberMap` (`JSONParserBPLibrary.AddMapNumber` (`JSONParserBPLibrary.AddMapNumber` (`JSONParserBPLibrary.MakeMapNumber` "X " (.x _impactnormal)) "Y" (.y _impactnormal)) "Z" (.z _impactnormal))))
  (bind _returnvalue_4 (`JSONParserBPLibrary.MakeJson_Object` (`JSONParserBPLibrary.AddMapObject` (`JSONParserBPLibrary.AddMapObject` (`JSONParserBPLibrary.MakeMapObject` "HIt Object" _returnvalue) "Hit Position" _returnvalue_2) "Hit Direction" _returnvalue_3)))
  (bind _returnvalue_5 (`JSONParserBPLibrary.JsonObjectToString` _returnvalue_4))
  (`KismetSystemLibrary.PrintString` _returnvalue_5 true true (struct :`G` 0.66 :`B` 1.0 :`A` 1.0) 10.0)
  (bind _asbp_game_instance (cast `/Game/Blueprints/Framework/BP_GameInstance` (`GameplayStatics.GetGameInstance`)))
  (bind _tcpconnection (`/Game/Blueprints/Framework/BP_GameInstance.TCPConnection` _asbp_game_instance))
  (bind _returnvalue_6 (`SocketClientBPLibrary.isTCPConnected` (`SocketClientBPLibrary.getSocketClientTarget`) _tcpconnection))
  (if _returnvalue_6
    (`SocketClientBPLibrary.socketClientSendTCP` :`self` (`SocketClientBPLibrary.getSocketClientTarget`) :`connectionID` _tcpconnection :`message` _returnvalue_5 :`addLineBreak` false)
    (`KismetSystemLibrary.PrintString` "Send" true true (struct :`R` 0.279998 :`G` 1.0 :`B` 0.022275 :`A` 1.0) 10.0)
    (else
      (`KismetSystemLibrary.PrintString` "Not connected." true true (struct :`R` 1.0 :`G` 0.120146 :`B` 0.060419 :`A` 1.0)))))

(event `self.ReceiveTick`
  (params (DeltaSeconds :type "Float (single-precision)"))
  (bind (_returnvalue_roll _returnvalue_pitch _returnvalue_yaw) (`KismetMathLibrary.BreakRotator` (`self.K2_GetActorRotation`)))
  (bind _springarm (`self.SpringArm`))
  (bind (_utmnorthing _utmeasting _utmzone) (`UTMConverter.LLtoUTM` (`self.RefLat`) (`self.RefLon`)))
  (bind (_utmnorthing_2 _utmeasting_2) (`UTMConverter.LLtoUTM` (`self.RefLat`) (`self.RefLon`)))
  (bind (_returnvalue_x _returnvalue_y _returnvalue_z) (`KismetMathLibrary.BreakVector` (/ (`self.K2_GetActorLocation`) (`self.UnitScaler`))))
  (bind (_utmnorthing_3 _utmeasting_3) (`UTMConverter.LLtoUTM` (`self.Lat`) (`self.Lon`)))
  (bind _returnvalue (`KismetStringLibrary.ParseIntoArray` (`KismetStringLibrary.Conv_DoubleToString` (`self.DataTime`)) "."))
  (bind (_lat _long) (`UTMConverter.UTMtoLL` (+ _utmnorthing _returnvalue_x) (+ _utmeasting _returnvalue_y) _utmzone))
  (bind (_returnvalue_x_2 _returnvalue_y_2 _returnvalue_z_2) (`KismetMathLibrary.BreakVector` (* (`KismetMathLibrary.MakeVector` (* -1 (- _utmeasting_2 _utmeasting_3)) (- _utmnorthing_2 _utmnorthing_3) (`self.Alt`)) (`self.UnitScaler`))))
  (if (`self.IsDemo`)
    (`KismetSystemLibrary.Delay` (`self.DelayTime`))
    (set `self.DataTime` (+ (`self.DataTime`) (`self.DelayTime`)))
    (set `self.OutData` (`KismetStringLibrary.Concat_StrStr` (`self.OutData`) (`KismetStringLibrary.Concat_StrStr` "PlatformData " "" (`KismetStringLibrary.Conv_IntToString` (`self.PlatformID`)) " " (`KismetStringLibrary.Concat_StrStr` (`KismetStringLibrary.Concat_StrStr` (`|GetArrayItem` _returnvalue) "." (`KismetStringLibrary.GetSubstring` (`|GetArrayItem` _returnvalue 1) 0 2)) " " (`KismetStringLibrary.Conv_DoubleToString` _lat) " " (`KismetStringLibrary.Conv_DoubleToString` _long) "  " (`KismetStringLibrary.Conv_DoubleToString` _returnvalue_z) " " (`KismetStringLibrary.Conv_DoubleToString` (+ _returnvalue_yaw 90.0)) " " (`KismetStringLibrary.Conv_DoubleToString` _returnvalue_pitch) " " (`KismetStringLibrary.Conv_DoubleToString` _returnvalue_roll) " \n"))))
    (else
      (`|ExecutionSequence`
        (:`then_0`
          ;[1 1 1] 카메라 조정
          (if (`self.CanCameraMove`)
            (bind _asbp_default_pawn_gps_a2s (cast `/Game/Blueprints/Framework/BP_DefaultPawn_GPS_A2S` (`GameplayStatics.GetPlayerPawn` 0)))
            (set `SpringArmComponent.TargetArmLength` (`KismetMathLibrary.FClamp` (+ (`SpringArmComponent.TargetArmLength` _springarm) (`/Game/Blueprints/Framework/BP_DefaultPawn_GPS_A2S.ZoomValue` _asbp_default_pawn_gps_a2s)) 100.0 20000.0) _springarm)
            (`SceneComponent.K2_SetRelativeRotation` (`self.SpringArm`) (`Controller.GetControlRotation` (`GameplayStatics.GetPlayerController` 0)) false false)))
        (:`then_1`
          (if (not (`self.IsHit`))
            (`self.K2_SetActorLocation` (`KismetMathLibrary.MakeVector` (.x (`KismetMathLibrary.MakeVector` _returnvalue_x_2 _returnvalue_y_2 _returnvalue_z_2)) (.y (`KismetMathLibrary.MakeVector` _returnvalue_x_2 _returnvalue_y_2 _returnvalue_z_2)) (.z (`KismetMathLibrary.MakeVector` _returnvalue_x_2 _returnvalue_y_2 _returnvalue_z_2))))
            (`self.K2_SetActorRotation` (`KismetMathLibrary.RLerp` (`self.K2_GetActorRotation`) (`KismetMathLibrary.MakeRotator` (+ (`self.Roll`) 0.0) (+ (`self.Pitch`) 0.0) (+ (`self.Yaw`) -90.0)) (`KismetMathLibrary.FClamp` (* DeltaSeconds 2.0)) true))))))))

(fn `UserConstructionScript`)