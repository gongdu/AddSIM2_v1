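; BP_KDX_II_2 is an actor, apparently a KDX-II warship, that animates its rotating antennas.
; Tick spins two antenna pivots about yaw at different fixed steps per frame, so their speed depends on frame rate.
; A delayed velocity threshold check in Tick leads to nothing.
; The Fire_Hampo event is empty, and an actor spawn at the Arrow transform is disconnected, with no class set.
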(event `self.ReceiveTick`
  (params (DeltaSeconds :type "Float (single-precision)"))
  (`SceneComponent.K2_AddRelativeRotation` (`self.Antenna_Pivot`) (struct :`Yaw` 5.0) false false)
  (`SceneComponent.K2_AddRelativeRotation` (`self.Antena_Main_Pivot`) (struct :`Yaw` 3.0) false false)
  (`KismetSystemLibrary.Delay` 0.2)
  (if (> (`KismetMathLibrary.VSize` (`self.GetVelocity`)) 50.0)
    _))

(event `Fire_Hampo`)

(event `Key|SpaceBar`
  (params (Key :type "Key Structure")))

(fn `UserConstructionScript`)