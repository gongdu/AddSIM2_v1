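; Actor that exports a SIMDIS ASCII Scenario Input (ASI) text log of platform data.
; Five seconds after BeginPlay, it builds a header block from each OutActors entry's ID, name and icon, prepending in reverse iteration to keep array order.
; It concatenates each entry's OutData, then saves scenario initialization, platform headers and data to Log2.txt through SaveTxt in a single write.
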(event `self.ReceiveBeginPlay`
  (`KismetSystemLibrary.Delay` 5.0)
  (bind (_arrayindex _arrayelement) (`/Engine/EditorBlueprintResources/StandardMacros.ReverseForEachLoop` (`self.Out Actors`))
    (:`LoopBody`
      (bind _returnvalue (`KismetStringLibrary.Conv_IntToString` (`/Game/Blueprints/BP_Node.PlatformID` _arrayelement)))
      (set `self.PlatformHeaderString` (`KismetStringLibrary.Concat_StrStr` (`KismetStringLibrary.Concat_StrStr` "PlatformID " _returnvalue " \n" "PlatformName " _returnvalue " \"" (`/Game/Blueprints/BP_Node.PlatformName` _arrayelement) "\" \n" "PlatformIcon " _returnvalue " \"" (`/Game/Blueprints/BP_Node.PlatformIcon` _arrayelement) "\" \n") (`self.PlatformHeaderString`))))
    (:`Completed`
      (for _array_element (`self.Out Actors`)
        (set `self.NodeData` (`KismetStringLibrary.Concat_StrStr` (`self.NodeData`) (`/Game/Blueprints/BP_Node.OutData` _array_element))))
      (`FileManagerBFL.SaveTxt` (`KismetStringLibrary.Concat_StrStr` (`KismetStringLibrary.Concat_StrStr` "# SIMDIS Ascii Scenario Input (ASI) File Format \n \n# Scenario Initialization \n \n" "Version " (`self.Version`) " \n" "RefLat " (`self.RefLat`) " \n" "RefLon " (`self.RefLon`) " \n" "CoordSystem \"LLA\" \nDegreeAngles 1 \n \n" "# Platform Header  \n \n" (`self.PlatformHeaderString`)) " \n# Platform Data \n \n \n# PlatformData PlatformID Time Lat Lon Alt Yow Pitch Roll  \n \n" (`self.NodeData`)) "Log2.txt"))))

(fn `UserConstructionScript`)